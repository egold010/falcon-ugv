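; UGV1BP is a drivable ground vehicle Blueprint that supports manual input and has an Autonomous flag.
; Throttle, brake and steering axes feed the VehicleMovementComponent only when Autonomous is off, while the handbrake action works regardless of that flag.
; Mouse camera control is inactive, as the mouse events are empty and the SpringArm rotation nodes are disconnected.
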(event EventBeginPlay)

(event Collision|EventActorBeginOverlap
  (params (OtherActor :type Actor%20Object%20Reference)))

(event EventTick
  (params (DeltaSeconds :type Float%20%28single-precision%29)))

(event Input|ActionEvents|InputActionHandbrake
  (params (Key :type Key%20Structure :default "None"))
  (bind _vehiclemovementcomponent (Variables|Default|GetVehicleMovementComponent))
  ;[0.15 0.15 0.15 0.5] Movement
  (:Pressed
    (Class|ChaosVehicleMovementComponent|SetHandbrakeInput _vehiclemovementcomponent true))
  (:Released
    (Class|ChaosVehicleMovementComponent|SetHandbrakeInput _vehiclemovementcomponent false)))

(event Input|AxisEvents|InputAxisThrottle
  (params (AxisValue :type Float%20%28single-precision%29))
  ;[0.15 0.15 0.15 0.5] Movement
  (if (not (Variables|Default|GetAutonomous))
    (Class|ChaosVehicleMovementComponent|SetThrottleInput (Variables|Default|GetVehicleMovementComponent) AxisValue)))

(event Input|AxisEvents|InputAxisBrake
  (params (AxisValue :type Float%20%28single-precision%29))
  ;[0.15 0.15 0.15 0.5] Movement
  (if (not (Variables|Default|GetAutonomous))
    (Class|ChaosVehicleMovementComponent|SetBrakeInput (Variables|Default|GetVehicleMovementComponent) AxisValue)))

(event Input|AxisEvents|InputAxisSteering
  (params (AxisValue :type Float%20%28single-precision%29))
  ;[0.15 0.15 0.15 0.5] Movement
  (if (not (Variables|Default|GetAutonomous))
    (Class|ChaosVehicleMovementComponent|SetSteeringInput (Variables|Default|GetVehicleMovementComponent) AxisValue)))

(event Input|MouseEvents|MouseX
  (params (AxisValue :type Float%20%28single-precision%29))
  ;[0.15 0.15 0.15 0.5] Camera
)

(event Input|MouseEvents|MouseY
  (params (AxisValue :type Float%20%28single-precision%29))
  ;[0.15 0.15 0.15 0.5] Camera
)

(fn ConstructionScript)